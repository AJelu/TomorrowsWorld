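; Simple rocket projectile Blueprint that adds flight and explosion effects to its parent class.
; BeginPlay spawns an attenuated flight sound at the rocket's location.
; PlayDeath plays the explosion sound, fires a force impulse, hides the mesh and trail, and activates explosion particles.
; It then starts a death timeline whose Finished event destroys the movement object and the rocket, delaying removal until the effects play.
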(event `self.ReceiveBeginPlay`
  (`parent.ReceiveBeginPlay`)
  (`GameplayStatics.SpawnSoundAtLocation` "/Game/Media/Sound/FX/Explosion/Rocket_fly_Cue.Rocket_fly_Cue" (0.0 0.0 0.0) (struct) 5.0 1.0 0.0 "/Game/Media/Sound/FX/Explosion/FireExplasion_SoundAttenuation.FireExplasion_SoundAttenuation" null))

(fn `PlayDeath`
  (bind _particlerocket (`self.ParticleRocket`))
  (`parent.PlayDeath`)
  (`GameplayStatics.SpawnSoundAtLocation` "/Game/Media/Sound/FX/Explosion/Explosion_Cue.Explosion_Cue" (0.0 0.0 0.0) (struct) 1.0 1.0 0.0 "/Game/Media/Sound/FX/Explosion/FireExplasion_SoundAttenuation.FireExplasion_SoundAttenuation" null)
  (`RadialForceComponent.FireImpulse` (`self.FireForce`))
  (`SceneComponent.SetVisibility` (`self.RocketMesh`) false false)
  (`ActorComponent.Activate` (`self.ParticleRocketExplosion`) true)
  (`ActorComponent.Deactivate` _particlerocket)
  (`SceneComponent.SetVisibility` _particlerocket false false)
  (`TimelineComponent.PlayFromStart` (`self.DethTimeLine`))
  (return))

(fn `UserConstructionScript`
  (`parent.UserConstructionScript`))