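; Base rocket actor that explodes on overlapping anything but its owning Character, stopping and destroying its separate Movement actor.
; SetMovement arms rocket collision, and SetCharacter sizes the blast sphere from that character's rocket stats.
; Detonation briefly enables the sphere's overlap events and forces an update, applying Power damage through DamageInterface.
; Remote instances loop ExplosionTimeLine to poll IsExplosion, then run PlayDeath.
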(event `self.ReceiveBeginPlay`
  (`/Engine/EditorBlueprintResources/ActorMacros.Switch Has Authority`
    (:`Remote`
      (`Timeline|ExplosionTimeLine` :!via `PlayFromStart`
        (:`Finished`
          (if (`self.IsExplosion`)
            (`self.PlayDeath`)
            (else
              (`TimelineComponent.PlayFromStart` (`self.ExplosionTimeLine`)))))))))

(event `self.Rocket.OnComponentBeginOverlap`
  (params (OverlappedComponent :type "PrimitiveComponent Object Reference") (OtherActor :type "Actor Object Reference") (OtherComp :type "PrimitiveComponent Object Reference") (OtherBodyIndex :type Integer) (bFromSweep :type Boolean) (SweepResult :type "HitResult Structure (by ref)"))
  (if (!= (`self.Character`) OtherActor)
    (`self.PlayDeath`)))

(event `self.Explosion.OnComponentBeginOverlap`
  (params (OverlappedComponent :type "PrimitiveComponent Object Reference") (OtherActor :type "Actor Object Reference") (OtherComp :type "PrimitiveComponent Object Reference") (OtherBodyIndex :type Integer) (bFromSweep :type Boolean) (SweepResult :type "HitResult Structure (by ref)"))
  (`/Engine/EditorBlueprintResources/StandardMacros.IsValid` (`self.Character`)
    (:`Is Valid`
      (bind _asdamage_interface (cast `/Game/Blueprints/Units/DamageInterface` OtherActor))
      (`/Game/Blueprints/Units/DamageInterface.DamageOnComponent` _asdamage_interface (`/Game/Blueprints/Units/CharactersStatsLogics.GetStatsRocket` (`self.Character`)) OtherComp self OverlappedComponent))))

(fn `ChangeColisionOnExplosion`
  (bind _explosion (`self.Explosion`))
  (set `PrimitiveComponent.bGenerateOverlapEvents` false (`self.Rocket`))
  (set `PrimitiveComponent.bGenerateOverlapEvents` true (`self.Explosion`))
  (`SphereComponent.SetSphereRadius` _explosion (`SphereComponent.SphereRadius` _explosion) true)
  (set `PrimitiveComponent.bGenerateOverlapEvents` false (`self.Explosion`))
  (set `self.IsExplosion` true)
  (return))

(fn `GetCharacter`
  (returns (Character :type "/Game/Blueprints/Units/CharactersStatsLogics Object Reference"))
  (return (`self.Character`)))

(fn `GetMovement`
  (returns (Movement :type "/Game/Blueprints/Rockets/SpiralMovement Object Reference"))
  (return (`self.Movement`)))

(fn `PlayDeath`
  (bind _movement (`self.Movement`))
  (`/Engine/EditorBlueprintResources/StandardMacros.IsValid` _movement
    (:`Is Valid`
      (`/Game/Blueprints/Rockets/SpiralMovement.StopMovement` _movement)
      (`self.K2_DestroyActor` _movement))
    (:`Is Not Valid`
      _))
  (`self.ChangeColisionOnExplosion`)
  (return))

(fn `SetCharacter`
  (params (Character :type "/Game/Blueprints/Units/CharactersStatsLogics Object Reference"))
  (bind _output_get (set `self.Character` Character))
  (`/Engine/EditorBlueprintResources/StandardMacros.IsValid` _output_get
    (:`Is Valid`
      (`SphereComponent.SetSphereRadius` (`self.Explosion`) (`.ExplosionDistance` (`/Game/Blueprints/Units/CharactersStatsLogics.GetStatsRocket` _output_get)) true))))

(fn `SetMovement`
  (params (Movement :type "/Game/Blueprints/Rockets/SpiralMovement Object Reference"))
  (set `self.Movement` Movement)
  (set `PrimitiveComponent.bGenerateOverlapEvents` true (`self.Rocket`)))

(fn `UserConstructionScript`)