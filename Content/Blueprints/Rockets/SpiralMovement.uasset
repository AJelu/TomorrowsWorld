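; SpiralMovement is a helper actor that flies a given rocket object along a narrowing spiral toward a target point.
; MoveToPoint stores the rocket and rebuilds LineSpline from the actor to that point.
; From BeginPlay, one timeline slides CircleSpline along the line while shrinking it, as another moves the rocket around that circle, producing the spiral.
; When travel finishes, StopCircle halts the circling and calls SelfDestroy, which is empty here.
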(event `StopCircle`
  (bind _rocketobject (`self.RocketObject`))
  (`|ExecutionSequence`
    (:`then_0`
      (bind (_direction _move) (`Timeline|CircleMoveTimeline` :!via `Stop` :!label _label)
        (:`Update`
          (`self.K2_SetActorTransform` _rocketobject (`KismetMathLibrary.MakeTransform` (.location (`SplineComponent.GetTransformAtTime` (`self.CircleSpline`) _move "World" false false)) (.rotation (`SplineComponent.GetTransformAtTime` (`self.CircleSpline`) _move "World" false false)) (`self.GetActorScale3D` _rocketobject)) false false))))
    (:`then_1`
      (`self.SelfDestroy`))))

(event `self.ReceiveBeginPlay`
  (`|ExecutionSequence`
    (:`then_0`
      (goto _label))
    (:`then_1`
      (bind (_direction _move) (`Timeline|TargetMoveTimeline`)
        (:`Update`
          (`SceneComponent.K2_SetRelativeTransform` (`self.CircleSpline`) (`SplineComponent.GetTransformAtTime` (`self.LineSpline`) _move "Local" false false) false false)
          (`SceneComponent.SetRelativeScale3D` (`self.CircleSpline`) (`KismetMathLibrary.Conv_DoubleToVector` (- 1.0 _move))))
        (:`Finished`
          (`self.StopCircle`))))))

(fn `MoveToPoint`
  (params (Point :type "Vector Structure") (CharacterWhoSend :type "/Game/Blueprints/Units/CharactersBaseLogics Object Reference") (RocketObjectRef :type "Actor Object Reference"))
  (bind _linespline (`self.LineSpline`))
  (set `self.Point` Point)
  (set `self.Character` CharacterWhoSend)
  (`/Engine/EditorBlueprintResources/StandardMacros.IsValid` RocketObjectRef
    (:`Is Valid`
      (set `self.RocketObject` RocketObjectRef)
      (`SplineComponent.ClearSplinePoints` _linespline false)
      (`SplineComponent.AddPoint` _linespline (make `SplinePoint` 0.0 (0.0 0.0 0.0) (0.0 0.0 0.0) (0.0 0.0 0.0) (struct) (1.0 1.0 1.0) "CurveCustomTangent") false)
      (`SplineComponent.AddPoint` _linespline (make `SplinePoint` 1.0 (- (`self.Point`) (`self.K2_GetActorLocation`)) (0.0 0.0 0.0) (0.0 0.0 0.0) (struct) (1.0 1.0 1.0) "CurveCustomTangent") true))))

(fn `SelfDestroy`)

(fn `UserConstructionScript`)