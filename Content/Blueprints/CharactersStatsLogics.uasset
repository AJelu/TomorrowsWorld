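; Actor Blueprint holding a character's stat logic for energy, condensator, speed, defense, kick, rocket and IA, all stored in CharacterInfo.
; UpdateStatsValue recomputes each stat from base plus item-level and CharacterType steps, and grouped getters expose the results.
; RecoverProcess applies timestamp-based regeneration, gating energy at a fraction of max, while UseCondencator spends charge and AddEnergy clamps changes, reporting overflow.
; Event graph is unused, so callers drive everything.
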(fn `AddEnergy`
  (params (SizeEnergy :type "Float (double-precision)"))
  (returns (Successful :type Boolean) (OutOfRange :type "Float (double-precision)"))
  (bind (_characterinfo_nickname _characterinfo_level _characterinfo_transform _characterinfo_charactertype _characterinfo_stats) (break `/Game/Data/Autorization/CharacterData` (`self.CharacterInfo`)))
  (bind (_characterinfo_nickname_2 _characterinfo_level_2 _characterinfo_transform_2 _characterinfo_charactertype_2 _characterinfo_stats_2) (break `/Game/Data/Autorization/CharacterData` (`self.CharacterInfo`)))
  (bind (_characterinfo_nickname_3 _characterinfo_level_3 _characterinfo_transform_3 _characterinfo_charactertype_3 _characterinfo_stats_3) (break `/Game/Data/Autorization/CharacterData` (`self.CharacterInfo`)))
  (bind (_characterinfo_nickname_4 _characterinfo_level_4 _characterinfo_transform_4 _characterinfo_charactertype_4 _characterinfo_stats_4) (break `/Game/Data/Autorization/CharacterData` (`self.CharacterInfo`)))
  (bind (_lasttimerecharge _energysizecurrent _energysizemax) (break `/Game/Data/Autorization/CharacterStats` _characterinfo_stats))
  (bind (_lasttimerecharge_2 _energysizecurrent_2 _energysizemax_2) (break `/Game/Data/Autorization/CharacterStats` _characterinfo_stats_2))
  (bind _returnvalue (+ SizeEnergy _energysizecurrent_2))
  (if (< _returnvalue 0.0)
    (`|VariableSetRef` (`.EnergySizeCurrent_104_B4DDDE3D4874054E6F864194489E0329` (break `/Game/Data/Autorization/CharacterStats` _characterinfo_stats_3)))
    (return false _returnvalue)
    (elif (> _returnvalue (`.Value_18_A88342054FD7F648EDD54F91339E9EFC` (break `/Game/Data/Autorization/StatsItem` _energysizemax_2)))
      (`|VariableSetRef` _energysizecurrent (`.Value_18_A88342054FD7F648EDD54F91339E9EFC` (break `/Game/Data/Autorization/StatsItem` _energysizemax)))
      (return false (- _returnvalue (`.Value_18_A88342054FD7F648EDD54F91339E9EFC` (break `/Game/Data/Autorization/StatsItem` _energysizemax))))
      (else
        (`|VariableSetRef` (`.EnergySizeCurrent_104_B4DDDE3D4874054E6F864194489E0329` (break `/Game/Data/Autorization/CharacterStats` _characterinfo_stats_4)) _returnvalue)
        (return true 0.0)))))

(fn `GetCondencator`
  (returns (Current :type "Float (double-precision)") (SizeMax :type "Float (double-precision)") (RecoverySpeed :type "Float (double-precision)"))
  (bind (_characterinfo_nickname _characterinfo_level _characterinfo_transform _characterinfo_charactertype _characterinfo_stats) (break `/Game/Data/Autorization/CharacterData` (`self.CharacterInfo`)))
  (bind (_lasttimerecharge _energysizecurrent _energysizemax _energyrecoverprocent _energyrecoverspeed _energyfullrecovertimeout _energyfullrecoverlastuse _condencatorsizecurrent _condencatorsizemax _condencatorrecoverspeed) (break `/Game/Data/Autorization/CharacterStats` _characterinfo_stats))
  (return _condencatorsizecurrent (`.Value_18_A88342054FD7F648EDD54F91339E9EFC` (break `/Game/Data/Autorization/StatsItem` _condencatorsizemax)) (`.Value_18_A88342054FD7F648EDD54F91339E9EFC` (break `/Game/Data/Autorization/StatsItem` _condencatorrecoverspeed))))

(fn `GetDefence`
  (returns (Armor :type "Float (double-precision)") (InBlock :type "Float (double-precision)"))
  (bind (_characterinfo_nickname _characterinfo_level _characterinfo_transform _characterinfo_charactertype _characterinfo_stats) (break `/Game/Data/Autorization/CharacterData` (`self.CharacterInfo`)))
  (bind (_lasttimerecharge _energysizecurrent _energysizemax _energyrecoverprocent _energyrecoverspeed _energyfullrecovertimeout _energyfullrecoverlastuse _condencatorsizecurrent _condencatorsizemax _condencatorrecoverspeed _speedwalk _speedrun _speedsuperrun _defensearmor _defenseinblock) (break `/Game/Data/Autorization/CharacterStats` _characterinfo_stats))
  (return (`.Value_18_A88342054FD7F648EDD54F91339E9EFC` (break `/Game/Data/Autorization/StatsItem` _defensearmor)) (`.Value_18_A88342054FD7F648EDD54F91339E9EFC` (break `/Game/Data/Autorization/StatsItem` _defenseinblock))))

(fn `GetEneergy`
  (returns (Current :type "Float (double-precision)") (SizeMax :type "Float (double-precision)") (RecoveryProcent :type "Float (double-precision)") (RecoverySpeed :type "Float (double-precision)") (FullRecoveryTimeout :type "Float (double-precision)") (FullRecoveryRestoredTime :type "Float (double-precision)") (FullRecoveryTrueUse :type Boolean))
  (bind (_characterinfo_nickname _characterinfo_level _characterinfo_transform _characterinfo_charactertype _characterinfo_stats) (break `/Game/Data/Autorization/CharacterData` (`self.CharacterInfo`)))
  (bind (_lasttimerecharge _energysizecurrent _energysizemax _energyrecoverprocent _energyrecoverspeed _energyfullrecovertimeout _energyfullrecoverlastuse) (break `/Game/Data/Autorization/CharacterStats` _characterinfo_stats))
  (bind (_valuebase _valuelevelcurrent _valuestepforitemlevel _valuestepforcharacterlevel _value) (break `/Game/Data/Autorization/StatsItem` _energyfullrecovertimeout))
  (bind _returnvalue (`KismetMathLibrary.GetTotalSeconds` (- (`KismetMathLibrary.Now`) _energyfullrecoverlastuse)))
  (return _energysizecurrent (`.Value_18_A88342054FD7F648EDD54F91339E9EFC` (break `/Game/Data/Autorization/StatsItem` _energysizemax)) (`.Value_18_A88342054FD7F648EDD54F91339E9EFC` (break `/Game/Data/Autorization/StatsItem` _energyrecoverprocent)) (`.Value_18_A88342054FD7F648EDD54F91339E9EFC` (break `/Game/Data/Autorization/StatsItem` _energyrecoverspeed)) _value _returnvalue (<= _value _returnvalue)))

(fn `GetIA`
  (returns (Level :type "Float (double-precision)") (Energy :type "Float (double-precision)"))
  (bind (_characterinfo_nickname _characterinfo_level _characterinfo_transform _characterinfo_charactertype _characterinfo_stats) (break `/Game/Data/Autorization/CharacterData` (`self.CharacterInfo`)))
  (bind (_lasttimerecharge _energysizecurrent _energysizemax _energyrecoverprocent _energyrecoverspeed _energyfullrecovertimeout _energyfullrecoverlastuse _condencatorsizecurrent _condencatorsizemax _condencatorrecoverspeed _speedwalk _speedrun _speedsuperrun _defensearmor _defenseinblock _kicksize _kicktimeoutmultiply _rocketpower _rocketspeed _rocketmaxdistancefly _rocketexplosiondistance _rocketrechargetimeout _rockettimeaiming _rocketgraduscorrection _ialevel _iaenergy) (break `/Game/Data/Autorization/CharacterStats` _characterinfo_stats))
  (return (`.Value_18_A88342054FD7F648EDD54F91339E9EFC` (break `/Game/Data/Autorization/StatsItem` _ialevel)) (`.Value_18_A88342054FD7F648EDD54F91339E9EFC` (break `/Game/Data/Autorization/StatsItem` _iaenergy))))

(fn `GetKick`
  (returns (Size :type "Float (double-precision)") (TimeoutMultiply :type "Float (double-precision)"))
  (bind (_characterinfo_nickname _characterinfo_level _characterinfo_transform _characterinfo_charactertype _characterinfo_stats) (break `/Game/Data/Autorization/CharacterData` (`self.CharacterInfo`)))
  (bind (_lasttimerecharge _energysizecurrent _energysizemax _energyrecoverprocent _energyrecoverspeed _energyfullrecovertimeout _energyfullrecoverlastuse _condencatorsizecurrent _condencatorsizemax _condencatorrecoverspeed _speedwalk _speedrun _speedsuperrun _defensearmor _defenseinblock _kicksize _kicktimeoutmultiply) (break `/Game/Data/Autorization/CharacterStats` _characterinfo_stats))
  (return (`.Value_18_A88342054FD7F648EDD54F91339E9EFC` (break `/Game/Data/Autorization/StatsItem` _kicksize)) (`.Value_18_A88342054FD7F648EDD54F91339E9EFC` (break `/Game/Data/Autorization/StatsItem` _kicktimeoutmultiply))))

(fn `GetRocket`
  (returns (Power :type "Float (double-precision)") (Speed :type "Float (double-precision)") (MaxDistanceFly :type "Float (double-precision)") (ExplosionDistance :type "Float (double-precision)") (RechargeTimeout :type "Float (double-precision)") (TimeAiming :type "Float (double-precision)") (GradusCorrection :type "Float (double-precision)"))
  (bind (_characterinfo_nickname _characterinfo_level _characterinfo_transform _characterinfo_charactertype _characterinfo_stats) (break `/Game/Data/Autorization/CharacterData` (`self.CharacterInfo`)))
  (bind (_lasttimerecharge _energysizecurrent _energysizemax _energyrecoverprocent _energyrecoverspeed _energyfullrecovertimeout _energyfullrecoverlastuse _condencatorsizecurrent _condencatorsizemax _condencatorrecoverspeed _speedwalk _speedrun _speedsuperrun _defensearmor _defenseinblock _kicksize _kicktimeoutmultiply _rocketpower _rocketspeed _rocketmaxdistancefly _rocketexplosiondistance _rocketrechargetimeout _rockettimeaiming _rocketgraduscorrection) (break `/Game/Data/Autorization/CharacterStats` _characterinfo_stats))
  (return (`.Value_18_A88342054FD7F648EDD54F91339E9EFC` (break `/Game/Data/Autorization/StatsItem` _rocketpower)) (`.Value_18_A88342054FD7F648EDD54F91339E9EFC` (break `/Game/Data/Autorization/StatsItem` _rocketspeed)) (`.Value_18_A88342054FD7F648EDD54F91339E9EFC` (break `/Game/Data/Autorization/StatsItem` _rocketmaxdistancefly)) (`.Value_18_A88342054FD7F648EDD54F91339E9EFC` (break `/Game/Data/Autorization/StatsItem` _rocketexplosiondistance)) (`.Value_18_A88342054FD7F648EDD54F91339E9EFC` (break `/Game/Data/Autorization/StatsItem` _rocketrechargetimeout)) (`.Value_18_A88342054FD7F648EDD54F91339E9EFC` (break `/Game/Data/Autorization/StatsItem` _rockettimeaiming)) (`.Value_18_A88342054FD7F648EDD54F91339E9EFC` (break `/Game/Data/Autorization/StatsItem` _rocketgraduscorrection))))

(fn `GetSpeed`
  (returns (Walk :type "Float (double-precision)") (Run :type "Float (double-precision)") (SuperRun :type "Float (double-precision)"))
  (bind (_characterinfo_nickname _characterinfo_level _characterinfo_transform _characterinfo_charactertype _characterinfo_stats) (break `/Game/Data/Autorization/CharacterData` (`self.CharacterInfo`)))
  (bind (_lasttimerecharge _energysizecurrent _energysizemax _energyrecoverprocent _energyrecoverspeed _energyfullrecovertimeout _energyfullrecoverlastuse _condencatorsizecurrent _condencatorsizemax _condencatorrecoverspeed _speedwalk _speedrun _speedsuperrun) (break `/Game/Data/Autorization/CharacterStats` _characterinfo_stats))
  (return (`.Value_18_A88342054FD7F648EDD54F91339E9EFC` (break `/Game/Data/Autorization/StatsItem` _speedwalk)) (`.Value_18_A88342054FD7F648EDD54F91339E9EFC` (break `/Game/Data/Autorization/StatsItem` _speedrun)) (`.Value_18_A88342054FD7F648EDD54F91339E9EFC` (break `/Game/Data/Autorization/StatsItem` _speedsuperrun))))

(fn `RecoverProcess`
  (locals (CallInterval :type "Float (double-precision)"))
  (bind (_characterinfo_nickname _characterinfo_level _characterinfo_transform _characterinfo_charactertype _characterinfo_stats) (break `/Game/Data/Autorization/CharacterData` (`self.CharacterInfo`)))
  (bind (_lasttimerecharge _energysizecurrent _energysizemax _energyrecoverprocent _energyrecoverspeed _energyfullrecovertimeout _energyfullrecoverlastuse _condencatorsizecurrent _condencatorsizemax _condencatorrecoverspeed) (break `/Game/Data/Autorization/CharacterStats` _characterinfo_stats))
  (set `local.CallInterval` (`KismetMathLibrary.GetTotalSeconds` (- _lasttimerecharge (`KismetMathLibrary.Now`))))
  (`|ExecutionSequence`
    (:`then_0`
      (`|VariableSetRef` _lasttimerecharge (`KismetMathLibrary.Now`)))
    (:`then_1`
      (if (< _energysizecurrent (* (`.Value_18_A88342054FD7F648EDD54F91339E9EFC` (break `/Game/Data/Autorization/StatsItem` _energysizemax)) (`.Value_18_A88342054FD7F648EDD54F91339E9EFC` (break `/Game/Data/Autorization/StatsItem` _energyrecoverprocent))))
        (`|VariableSetRef` _energysizecurrent (+ _energysizecurrent (* (`local.CallInterval`) (`.Value_18_A88342054FD7F648EDD54F91339E9EFC` (break `/Game/Data/Autorization/StatsItem` _energyrecoverspeed)))))))
    (:`then_2`
      (if (< _condencatorsizecurrent (`.Value_18_A88342054FD7F648EDD54F91339E9EFC` (break `/Game/Data/Autorization/StatsItem` _condencatorsizemax)))
        (`|VariableSetRef` _condencatorsizecurrent (+ _condencatorsizecurrent (* (`local.CallInterval`) (`.Value_18_A88342054FD7F648EDD54F91339E9EFC` (break `/Game/Data/Autorization/StatsItem` _condencatorrecoverspeed)))))))))

(fn `UpdateStatsValue`
  (bind (_characterinfo_nickname _characterinfo_level _characterinfo_transform _characterinfo_charactertype _characterinfo_stats) (break `/Game/Data/Autorization/CharacterData` (`self.CharacterInfo`)))
  (bind (_lasttimerecharge _energysizecurrent _energysizemax _energyrecoverprocent _energyrecoverspeed _energyfullrecovertimeout _energyfullrecoverlastuse _condencatorsizecurrent _condencatorsizemax _condencatorrecoverspeed _speedwalk _speedrun _speedsuperrun _defensearmor _defenseinblock _kicksize _kicktimeoutmultiply _rocketpower _rocketspeed _rocketmaxdistancefly _rocketexplosiondistance _rocketrechargetimeout _rockettimeaiming _rocketgraduscorrection _ialevel _iaenergy) (break `/Game/Data/Autorization/CharacterStats` _characterinfo_stats))
  (`self.UpdateValue` _energysizemax)
  (`self.UpdateValue` _energyrecoverprocent)
  (`self.UpdateValue` _energyrecoverspeed)
  (`self.UpdateValue` _energyfullrecovertimeout)
  (`self.UpdateValue` _condencatorsizemax)
  (`self.UpdateValue` _condencatorrecoverspeed)
  (`self.UpdateValue` _speedwalk)
  (`self.UpdateValue` _speedrun)
  (`self.UpdateValue` _speedsuperrun)
  (`self.UpdateValue` _defensearmor)
  (`self.UpdateValue` _defenseinblock)
  (`self.UpdateValue` _kicksize)
  (`self.UpdateValue` _kicktimeoutmultiply)
  (`self.UpdateValue` _rocketpower)
  (`self.UpdateValue` _rocketspeed)
  (`self.UpdateValue` _rocketmaxdistancefly)
  (`self.UpdateValue` _rocketexplosiondistance)
  (`self.UpdateValue` _rocketrechargetimeout)
  (`self.UpdateValue` _rockettimeaiming)
  (`self.UpdateValue` _rocketgraduscorrection)
  (`self.UpdateValue` _ialevel)
  (`self.UpdateValue` _iaenergy))

(fn `UpdateValue`
  (params (Info :type "/Game/Data/Autorization/StatsItem Structure (by ref)"))
  (bind (_valuebase _valuelevelcurrent _valuestepforitemlevel _valuestepforcharacterlevel _value) (break `/Game/Data/Autorization/StatsItem` Info))
  (bind (_characterinfo_nickname _characterinfo_level _characterinfo_transform _characterinfo_charactertype) (break `/Game/Data/Autorization/CharacterData` (`self.CharacterInfo`)))
  (`|VariableSetRef` _value (+ _valuebase (* _valuelevelcurrent _valuestepforitemlevel) (* _characterinfo_charactertype _valuestepforcharacterlevel)))
  (return))

(fn `UseCondencator`
  (params (UseedSize :type "Float (double-precision)"))
  (returns (Successful :type Boolean))
  (bind (_characterinfo_nickname _characterinfo_level _characterinfo_transform _characterinfo_charactertype _characterinfo_stats) (break `/Game/Data/Autorization/CharacterData` (`self.CharacterInfo`)))
  (bind (_lasttimerecharge _energysizecurrent _energysizemax _energyrecoverprocent _energyrecoverspeed _energyfullrecovertimeout _energyfullrecoverlastuse _condencatorsizecurrent) (break `/Game/Data/Autorization/CharacterStats` _characterinfo_stats))
  (if (and (>= UseedSize 0.0) (<= UseedSize _condencatorsizecurrent))
    (`|VariableSetRef` _condencatorsizecurrent (- _condencatorsizecurrent UseedSize))
    (return true)
    (else
      (return false))))

(fn `UserConstructionScript`
  (`parent.UserConstructionScript`))