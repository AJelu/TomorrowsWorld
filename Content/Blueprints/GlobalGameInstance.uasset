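; Game instance that holds player accounts, login and connection state, and shared lookup data across levels.
; It loads the SavingGameData slot on init and saves it on shutdown with the password blanked.
; Setup functions reset session state for connecting, registering or starting a server, the last taking the first player's characters.
; It also links the viewed character to the level widget and serves stat, item, skill and combo info.
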(event `self.ReceiveInit`
  (bind _returnvalue (`GameplayStatics.LoadGameFromSlot` "ServerData"))
  (bind _assaving_game_data (cast `/Game/Data/SavingGameData` _returnvalue))
  (set `self.Players` (`/Game/Data/SavingGameData.Players` _assaving_game_data))
  (set `self.MyLoginPassword` (`/Game/Data/SavingGameData.LastWritedMyLoginPassword` _assaving_game_data))
  (set `self.ConnectIP` (`/Game/Data/SavingGameData.LastWritedConnectIP` _assaving_game_data)))

(event `self.ReceiveShutdown`
  (bind _returnvalue (`GameplayStatics.CreateSaveGameObject` "/Game/Data/SavingGameData.SavingGameData_C"))
  (set `/Game/Data/SavingGameData.Players` (`self.Players`) _returnvalue)
  (`|VariableSetRef` (`.Password_4_7D902B95494F24FF8A0A618A3B352FFD` (break `/Game/Data/Autorization/LoginPassword` (`self.MyLoginPassword`))))
  (set `/Game/Data/SavingGameData.LastWritedMyLoginPassword` (`self.MyLoginPassword`) _returnvalue)
  (set `/Game/Data/SavingGameData.LastWritedConnectIP` (`self.ConnectIP`) _returnvalue)
  (`GameplayStatics.SaveGameToSlot` _returnvalue "ServerData"))

(event `SetCharacterToViewWiget`
  (params (Character :type "/Game/Blueprints/Units/CharactersStatsLogics Object Reference (by ref)"))
  (`/Engine/EditorBlueprintResources/StandardMacros.IsValid` Character
    (:`Is Valid`
      (set `self.Character` Character)
      (`/Engine/EditorBlueprintResources/StandardMacros.IsValid` (`self.GameLevelWiget`)
        (:`Is Valid`
          (`/Game/UI/WidgetBlueprint/GameLevel/GameLevelWigetBluePrint.SetCharacterToView` (`self.GameLevelWiget`) (`self.Character`)))))))

(event `SetGameLevelWiget`
  (params (GameLevelWiget :type "/Game/UI/WidgetBlueprint/GameLevel/GameLevelWigetBluePrint Object Reference (by ref)"))
  (`/Engine/EditorBlueprintResources/StandardMacros.IsValid` GameLevelWiget
    (:`Is Valid`
      (set `self.GameLevelWiget` GameLevelWiget)
      (`/Engine/EditorBlueprintResources/StandardMacros.IsValid` (`self.Character`)
        (:`Is Valid`
          (`/Game/UI/WidgetBlueprint/GameLevel/GameLevelWigetBluePrint.SetCharacterToView` (`self.GameLevelWiget`) (`self.Character`)))))))

(fn `GetInfoBagItem`
  (params (BagItem :type "/Game/Data/Bag/BagItemsEnum Enum" :default "NewEnumerator0"))
  (returns (Info :type "/Game/Data/ItemInfo Structure") (Good :type Boolean))
  (bind (_value _returnvalue) (`BlueprintMapLibrary.Map_Find` (`self.BagItemInfo`) BagItem))
  (return _value _returnvalue))

(fn `GetInfoCombo`
  (params (CharacterIndex :type Integer) (ComboButtonIndex :type Integer))
  (returns (Info :type "/Game/Data/ItemInfo Structure") (Good :type Boolean))
  (bind _items (break `/Game/Data/ManyItemInfo` (`|GetArrayItem` (`self.ComboInfo`) (`local.CharacterIndex`))))
  (if (< (`local.CharacterIndex`) (`KismetArrayLibrary.Array_Length` (`self.ComboInfo`)))
    (if (< (`local.ComboButtonIndex`) (`KismetArrayLibrary.Array_Length` _items))
      (return (`|GetArrayItem` _items (`local.ComboButtonIndex`)) true)
      (else
        _)))
  (return (struct) false))

(fn `GetInfoSkill`
  (params (Skill :type "/Game/Data/Skills/SkillsEnum Enum" :default "NewEnumerator4"))
  (returns (Info :type "/Game/Data/ItemInfo Structure") (Good :type Boolean))
  (bind (_value _returnvalue) (`BlueprintMapLibrary.Map_Find` (`self.SkillsInfo`) Skill))
  (return _value _returnvalue))

(fn `GetInfoStat`
  (params (Stat :type "/Game/Data/Stats/StatsEnum Enum" :default "NewEnumerator24"))
  (returns (Info :type "/Game/Data/ItemInfo Structure") (Good :type Boolean))
  (bind (_value _returnvalue) (`BlueprintMapLibrary.Map_Find` (`self.StatsInfo`) Stat))
  (return _value _returnvalue))

(fn `SetConnectData`
  (params (MyLoginPassword :type "/Game/Data/Autorization/LoginPassword Structure") (ConnectIP :type String))
  (set `self.MyLoginPassword` MyLoginPassword)
  (set `self.ConnectIP` ConnectIP)
  (`KismetArrayLibrary.Array_Clear` (`self.MyCharacter`))
  (set `self.SelectedCharacter` -1)
  (set `self.RegistrationState` 0)
  (set `self.BadLoginingShowinMainLevel` false)
  (set `self.NeedSpawnCharacterForServer` true))

(fn `SetRegistrationData`
  (params (MyLoginPassword :type "/Game/Data/Autorization/LoginPassword Structure") (ConnectIP :type String))
  (set `self.MyLoginPassword` MyLoginPassword)
  (set `self.ConnectIP` ConnectIP)
  (`KismetArrayLibrary.Array_Clear` (`self.MyCharacter`))
  (set `self.SelectedCharacter` -1)
  (set `self.RegistrationState` 1)
  (set `self.BadLoginingShowinMainLevel` false)
  (set `self.NeedSpawnCharacterForServer` true))

(fn `SetStartServerData`
  (bind _mycharacter (`self.MyCharacter`))
  (bind (_output_loginpassword _output_chars) (break `/Game/Data/Autorization/UserAccount` (`|GetArrayItem` (`self.Players`))))
  (set `self.MyLoginPassword` (make `/Game/Data/Autorization/LoginPassword` ""))
  (set `self.ConnectIP` "")
  (`KismetArrayLibrary.Array_Clear` _mycharacter)
  (`KismetArrayLibrary.Array_Append` _mycharacter _output_chars)
  (set `self.SelectedCharacter` -1)
  (set `self.RegistrationState` 0)
  (set `self.BadLoginingShowinMainLevel` false)
  (set `self.NeedSpawnCharacterForServer` true))