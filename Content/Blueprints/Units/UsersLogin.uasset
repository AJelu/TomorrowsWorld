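; UsersLogin is the client-server login pawn that registers players, authenticates them and swaps itself for their selected character.
; The server checks credentials against GameInstance player records, logs out duplicate sessions, overwrites stored characters with the client's list, then spawns, possesses and ground-adjusts the character.
; Client events store results in GameInstance and open the main or character-choice level.
; On EndPlay, the server saves the character's transform to its record.
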(event `self.ReceiveBeginPlay`
  (bind _gameinstans (`self.GameInstans`))
  (bind _gameinstans_2 (`self.GameInstans`))
  (bind (_myloginpassword_login _myloginpassword_password) (break `/Game/Data/Autorization/LoginPassword` (`/Game/Blueprints/GlobalGameInstance.MyLoginPassword` _gameinstans)))
  (bind (_myloginpassword_login_2 _myloginpassword_password_2) (break `/Game/Data/Autorization/LoginPassword` (`/Game/Blueprints/GlobalGameInstance.MyLoginPassword` (`self.GameInstans`))))
  (bind (_myloginpassword_login_3 _myloginpassword_password_3) (break `/Game/Data/Autorization/LoginPassword` (`/Game/Blueprints/GlobalGameInstance.MyLoginPassword` (`self.GameInstans`))))
  ;[1 1 1] Player initialization
  (bind _asglobal_game_instance (cast `/Game/Blueprints/GlobalGameInstance` (`GameplayStatics.GetGameInstance`)))
  (set `self.GameInstans` _asglobal_game_instance)
  (if (`self.UsingClientServerLogic`)
    (`/Engine/EditorBlueprintResources/ActorMacros.Switch Has Authority`
      (:`Authority`
        ;[1 1 1] Server copies logic
        (if (`/Game/Blueprints/GlobalGameInstance.NeedSpawnCharacterForServer` _gameinstans_2)
          (set `/Game/Blueprints/GlobalGameInstance.NeedSpawnCharacterForServer` false _gameinstans_2)
          ;[1 1 1] Client copies logic
          ;;[0.7814 1 0.6626] Logining
          (if (not (`self.Teleport`)) :!label _label
            (`self.ConnectClientToServer` _myloginpassword_login _myloginpassword_password (`/Game/Blueprints/GlobalGameInstance.SelectedCharacter` _gameinstans) (`/Game/Blueprints/GlobalGameInstance.MyCharacters` _gameinstans)))))
      (:`Remote`
        (if (not (and (`KismetStringLibrary.NotEqual_StrStr` _myloginpassword_login_2) (`KismetStringLibrary.NotEqual_StrStr` _myloginpassword_password_2)))
          (`GameplayStatics.OpenLevelBySoftObjectPtr` "/Game/Levels/MainLevel/MainLevel.MainLevel")
          (elif (== (`/Game/Blueprints/GlobalGameInstance.RegistrationState` (`self.GameInstans`)) 0)
            (goto _label)
            (else
              ;;[0.3229 0.5839 1] Registration
              (`self.RegisterNewPlayer` _myloginpassword_login_3 _myloginpassword_password_3))))))))

(event `SetCharacterToShowUi`
  (`KismetSystemLibrary.PrintString` "SetCharacter")
  (bind _asglobal_game_instance (cast `/Game/Blueprints/GlobalGameInstance` (`GameplayStatics.GetGameInstance`)))
  (bind _ascharacters_stats_logics (cast `/Game/Blueprints/Units/CharactersStatsLogics` self))
  (`/Game/Blueprints/GlobalGameInstance.SetCharacterToViewWiget` _asglobal_game_instance _ascharacters_stats_logics))

(event `ConnectClientToServer`
  (params (Login :type String) (Password :type String) (Character :type Integer) (Characters :type "Array of /Game/Data/CharacterData Structure"))
  (bind _templocation (`self.TempLocation`))
  ;[0.7847 1 0.7763] Server logic
  ;;[0 0.003062 1] Autorize on server
  (bind (_finded _characters _password _online _recorditem) (`self.FindUser` Login Password))
  (if (and _finded _password)
    (if (not (not _online))
      (`self.DisconnectUser` _recorditem))
    (if (and (> (`KismetArrayLibrary.Array_Length` Characters) 0) (>= Character 0))
      (set `self.IndexUserRecord` _recorditem)
      (set `self.IndexCharacter` Character)
      ;;[0 1 0.1088] Logining successful and spawn need characters
      (`self.Rewrite Characters List` Characters (`self.IndexUserRecord`))
      (`KismetSystemLibrary.Delay` 1.0)
      (bind (_goodrespawn _newactor _transform) (`self.RespawnCharacter` (`self.IndexCharacter`)))
      (`self.SetCharacterToShowUi` _newactor)
      (set `self.TempLocation` (.location _transform))
      (while (!= (`self.TempLoop`) 0)
        ;;[1 1 1] Checking place good for spawn (exist object under new actor)
        (`/Engine/EditorBlueprintResources/StandardMacros.DecrementInt` (`self.TempLoop`)
          (:`  `
            (bind (_outhit _returnvalue) (`KismetSystemLibrary.LineTraceSingle` (+ _templocation (0.0 0.0 -200.0)) (+ _templocation (0.0 0.0 -10000.0)) "TraceTypeQuery1"))
            (if _returnvalue
              (set `self.TempLoop` 0)
              (else
                (set `self.TempLocation` (+ (0.0 0.0 500.0) _templocation)))))))
      (`self.K2_SetActorTransform` _newactor (`KismetMathLibrary.MakeTransform` (`self.TempLocation`) (.rotation _transform) (.scale _transform)) false false)
      (`self.K2_DestroyActor`)
      (else
        ;;[1 0.8792 0] Logining successful and send characters to client for choise
        (`self.ConnectionSuccessfulChoiseCharacters` _characters)))
    (else
      ;;[1 0.01705 0] Not foud user or bad password
      (`self.ConnectionError`))))

(event `RegisterNewPlayer`
  (params (Login :type String) (Password :type String))
  ;[0.7847 1 0.7763] Server logic
  ;;[1 1 1] Registration
  (bind _finded (`self.FindUser` Login Password))
  (if _finded
    (`self.RegistrationError`)
    (else
      (`KismetArrayLibrary.Array_Add` (`/Game/Blueprints/GlobalGameInstance.Players` (`self.GameInstans`)) (make `/Game/Data/Autorization/UserAccount` (make `/Game/Data/Autorization/LoginPassword` Login Password)))
      (`KismetSystemLibrary.PrintString` "Registered")
      (`self.RegistrationSuccessful`))))

(event `ConnectionSuccessfulChoiseCharacters`
  (params (Characters :type "Array of /Game/Data/CharacterData Structure"))
  ;[0.6756 0.7426 1] Client logic
  ;;[1 0.8659 0] Logining successful and send characters to client for choise
  (set `/Game/Blueprints/GlobalGameInstance.MyCharacters` Characters (`self.GameInstans`))
  (`GameplayStatics.OpenLevelBySoftObjectPtr` "/Game/Levels/ChoiceLevel/ChoiceLevel.ChoiceLevel"))

(event `ConnectionError`
  ;[0.6756 0.7426 1] Client logic
  ;;[1 0 0.05666] Not foud user or bad password
  (set `/Game/Blueprints/GlobalGameInstance.BadLoginingShowinMainLevel` true (`self.GameInstans`))
  (`GameplayStatics.OpenLevelBySoftObjectPtr` "/Game/Levels/MainLevel/MainLevel.MainLevel"))

(event `RegistrationSuccessful`
  ;[0.6756 0.7426 1] Client logic
  ;;[1 1 1] Registration
  (set `/Game/Blueprints/GlobalGameInstance.RegistrationState` 1 (`self.GameInstans`))
  (`GameplayStatics.OpenLevelBySoftObjectPtr` "/Game/Levels/MainLevel/MainLevel.MainLevel" :!label _label_2))

(event `RegistrationError`
  ;[0.6756 0.7426 1] Client logic
  ;;[1 1 1] Registration
  (set `/Game/Blueprints/GlobalGameInstance.RegistrationState` -1 (`self.GameInstans`))
  (goto _label_2))

(event `LogoutOnlineUser`
  ;[0.6756 0.7426 1] Client logic
  ;;[1 1 1] LogOut
  (`GameplayStatics.OpenLevelBySoftObjectPtr` "/Game/Levels/MainLevel/MainLevel.MainLevel" :!label _label_3))

(event `Key|R`
  (params (Key :type "Key Structure"))
  (:`Released`
    (goto _label_3)))

(event `self.ReceiveEndPlay`
  (params (EndPlayReason :type "EEndPlayReason Enum" :default "Destroyed"))
  (bind (_characterinfo_nickname _characterinfo_level _characterinfo_transform) (break `/Game/Data/CharacterData` (`self.CharacterInfo`)))
  ;[1 1 1] SaveInformation
  (`/Engine/EditorBlueprintResources/ActorMacros.Switch Has Authority`
    (:`Authority`
      (if (and (>= (`self.IndexUserRecord`) 0) (>= (`self.IndexCharacter`) 0))
        (`|VariableSetRef` _characterinfo_transform (`KismetMathLibrary.MakeTransform` (+ (.location (`self.GetTransform`)) (0.0 0.0 10.0)) (.rotation (`self.GetTransform`)) (.scale (`self.GetTransform`))))
        (`KismetArrayLibrary.Array_Set` (`.Chars_7_EE6EC6454E5394E0289F8282CF215DD3` (break `/Game/Data/Autorization/UserAccount` (`|GetArrayItem` (`/Game/Blueprints/GlobalGameInstance.Players` (`self.GameInstans`)) (`self.IndexUserRecord`)))) (`self.IndexCharacter`) (`self.CharacterInfo`))))))

(fn `DisconnectUser`
  (params (UserRecordItem :type Integer))
  (locals (Controller_ :type "Controller Object Reference"))
  (bind (_output_loginpassword _output_chars _output_online _output_pawn) (break `/Game/Data/Autorization/UserAccount` (`|GetArrayItem` (`/Game/Blueprints/GlobalGameInstance.Players` (`self.GameInstans`)) UserRecordItem)))
  (if (`KismetSystemLibrary.IsValid` _output_pawn)
    (`|VariableSetRef` _output_online)
    (`self.LogoutOnlineUser` _output_pawn)
    (return)))

(fn `FindUser`
  (params (Login :type String) (PasswordCompare :type String))
  (returns (Finded :type Boolean) (Characters :type "Array of /Game/Data/CharacterData Structure") (Password :type Boolean) (Online :type Boolean) (RecordItem :type Integer))
  (if true
    (for (_array_element _array_index) (`/Game/Blueprints/GlobalGameInstance.Players` (`self.GameInstans`))
      (bind (_login _password) (break `/Game/Data/Autorization/LoginPassword` (break `/Game/Data/Autorization/UserAccount` _array_element)))
      (if (`KismetStringLibrary.EqualEqual_StrStr` Login _login)
        (return true (`.Chars_7_EE6EC6454E5394E0289F8282CF215DD3` (break `/Game/Data/Autorization/UserAccount` _array_element)) (`KismetStringLibrary.EqualEqual_StrStr` _password PasswordCompare) (`.Online_9_40C245584D76A34728FD9C91CE379B80` (break `/Game/Data/Autorization/UserAccount` _array_element)) _array_index))))
  (return false _ false false -1))

(fn `RespawnCharacter`
  (params (IndexCharacter :type Integer))
  (returns (GoodRespawn :type Boolean) (NewActor :type "/Game/Blueprints/Units/UsersLogin Object Reference") (Transform :type "Transform Structure"))
  (locals (SpawnClass :type "/Game/Blueprints/Units/UsersLogin Class Reference") (CharacterData :type "/Game/Data/CharacterData Structure"))
  (bind (_output_loginpassword _output_chars _output_online _output_pawn) (break `/Game/Data/Autorization/UserAccount` (`|GetArrayItem` (`/Game/Blueprints/GlobalGameInstance.Players` (`self.GameInstans`)) (`self.IndexUserRecord`))))
  (bind (_output_loginpassword_2 _output_chars_2) (break `/Game/Data/Autorization/UserAccount` (`|GetArrayItem` (`/Game/Blueprints/GlobalGameInstance.Players` (`self.GameInstans`)) (`self.IndexUserRecord`))))
  (if (and (>= IndexCharacter 0) (< IndexCharacter (`KismetArrayLibrary.Array_Length` _output_chars_2)))
    (bind _output_get (set `local.CharacterData` (`|GetArrayItem` _output_chars_2 IndexCharacter)))
    (bind ((`Transform_16_404AA43F42F49BD35CD1D890559FE1B8` _transform) (`CharacterType_10_7B41A4CA43C8C74C0334C8B90A9B93A3` _charactertype)) (break `/Game/Data/CharacterData` _output_get))
    (switch `int` _charactertype
      (:`Default`
        (set `local.SpawnClass` "UsersLogin_C"))
      (:`0`
        (set `local.SpawnClass` "/Game/Blueprints/Units/Hero/Crux/Crux_Player_Character.Crux_Player_Character_C"))
      (:`1`
        (set `local.SpawnClass` "/Game/Blueprints/Units/Hero/Fornax/Fornax_Player_Character.Fornax_Player_Character_C"))
      (:`2`
        (set `local.SpawnClass` "/Game/Blueprints/Units/Hero/Lynx/Lynx_Player_Character.Lynx_Player_Character_C")))
    (bind _returnvalue (`|SpawnActorFromClass` (`local.SpawnClass`) _transform "Undefined" "OverrideRootScale" (`self.GetController`) null))
    (set `/Game/Blueprints/Units/UsersLogin.Teleport` true _returnvalue)
    (set `/Game/Blueprints/Units/UsersLogin.CharacterInfo` (`local.CharacterData`) _returnvalue)
    (set `/Game/Blueprints/Units/UsersLogin.UsingClientServerLogic` true _returnvalue)
    (`Controller.Possess` (`self.GetController`) _returnvalue)
    (`|VariableSetRef` _output_online true)
    (`|VariableSetRef` _output_pawn _returnvalue)
    (set `/Game/Blueprints/Units/UsersLogin.IndexUserRecord` (`self.IndexUserRecord`) _returnvalue)
    (set `self.IndexUserRecord` -1)
    (set `/Game/Blueprints/Units/UsersLogin.IndexCharacter` (`self.IndexCharacter`) _returnvalue)
    (set `self.IndexCharacter` -1)
    (return true _returnvalue _transform)
    (else
      (return false null))))

(fn `Rewrite Characters List`
  (params (NewCharacters :type "Array of /Game/Data/CharacterData Structure") (IndexUserRecord :type Integer))
  (bind (_output_loginpassword _output_chars) (break `/Game/Data/Autorization/UserAccount` (`|GetArrayItem` (`/Game/Blueprints/GlobalGameInstance.Players` (`self.GameInstans`)) IndexUserRecord)))
  (`KismetArrayLibrary.Array_Clear` _output_chars)
  (`KismetArrayLibrary.Array_Append` _output_chars NewCharacters)
  (return))

(fn `UserConstructionScript`)