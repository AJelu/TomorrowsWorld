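; Character Blueprint layer that owns a unit's progression and resources in CharacterInfo: stats, energy, condensator, bag items, skills and combos.
; Stat values derive from base, stat level and character level, with upgrades spending DarkEnergy or IAPatches.
; A looping timeline runs Process, regenerating energy and condensator from elapsed timestamps on authority.
; Mutations are authority-gated, with player actions forwarded through Server events and widgets refreshed locally or through Client events.
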(event `self.ReceiveBeginPlay`
  (`parent.ReceiveBeginPlay`)
  (`Timeline|UpdateEnergy` :!via `PlayFromStart`
    (:`Finished`
      (`TimelineComponent.PlayFromStart` (`self.UpdateEnergy`))
      (`self.Process`)
      (if (`self.NeedUpdateUI`)
        (`self.UIUpdated`)
        (`self.UpdateStatsWiget`)
        (`self.UpdateBagWiget`)
        (`self.UpdateUserInfoWiget`)
        (`self.UpdateIAWiget`)))))

(event `ServerAddLevelStatsGroupByIndex`
  (params (Index :type Integer))
  (`self.AddLevelStatsGroupByIndex` Index)
  (`self.ClientUpdateStatsWiget`)
  (`self.ClientUpdateBagWiget`)
  (`self.ClientUpdateUserInfoWiget`))

(event `ServerUseBagItem`
  (params (Name :type "/Game/Data/Bag/BagItemsEnum Enum" :default "NewEnumerator0"))
  (`self.UseBagItem` Name)
  (`self.ClientUpdateBagWiget`)
  (`self.ClientUpdateBagWiget`))

(event `ServerAddAllowedCombo`
  (params (Index :type Integer))
  (`self.AddAllowedCombo` Index)
  (`self.ClientUpdateIAWiget`)
  (`self.ClientUpdateBagWiget`))

(event `ServerAddSkillLevel`
  (params (Skill :type "/Game/Data/Skills/SkillsEnum Enum" :default "NewEnumerator0"))
  (`self.AddSkillLevel` Skill)
  (`self.ClientUpdateIAWiget`)
  (`self.ClientUpdateBagWiget`))

(event `UIUpdated`
  (set `self.NeedUpdateUI` false))

(event `ClientUpdateStatsWiget`
  ;[1 1 1] Client Updates
  (`self.UpdateStatsWiget`))

(event `ClientUpdateBagWiget`
  ;[1 1 1] Client Updates
  (`self.UpdateBagWiget`))

(event `ClientUpdateUserInfoWiget`
  ;[1 1 1] Client Updates
  (`self.UpdateUserInfoWiget`))

(event `ClientUpdateIAWiget`
  ;[1 1 1] Client Updates
  (`self.UpdateIAWiget`))

(fn `AddAllowedCombo`
  (params (Index :type Integer))
  (bind ((`PointRespawn_82_55D78C5C4C9C365BBAFF1F9AE69BA5F7` _pointrespawn) (`AllowedCombo_66_05522F344A4CF73CFAD1E4AE25DFB917` _allowedcombo)) (break `/Game/Data/CharacterData1` (`self.CharacterInfo`)))
  (bind ((`PointRespawn_82_55D78C5C4C9C365BBAFF1F9AE69BA5F7` _pointrespawn_2) (`IAPatches_35_C3979C3E43A2FE95F15DE98B41BFD762` _iapatches)) (break `/Game/Data/CharacterData1` (`self.CharacterInfo`)))
  (bind _output (`|GetArrayItem` _allowedcombo (`local.Index`)))
  (`/Engine/EditorBlueprintResources/ActorMacros.Switch Has Authority`
    (:`Authority`
      (if (> _iapatches 0)
        (if (< (`local.Index`) (`KismetArrayLibrary.Array_Length` _allowedcombo))
          (if (> (`KismetArrayLibrary.Array_Length` (`.Combo_8_9C06713E4099F8A91F2E29B53A67213C` (break `/Game/Data/Combo/ComboLevels` (`|GetArrayItem` (`self.ComboByLevelAnimList`) (`local.Index`))))) _output)
            (`/Engine/EditorBlueprintResources/StandardMacros.IncrementInt` _output
              (:`  `
                (`/Engine/EditorBlueprintResources/StandardMacros.DecrementInt` _iapatches
                  (:`  `
                    (`self.UpdateIAWiget`)
                    (`self.UpdateBagWiget`)))))))))
    (:`Remote`
      (`self.ServerAddAllowedCombo` Index))))

(fn `AddedEnergy`
  (params (CurrentEnergy :type "Float (double-precision)") (PreviouslyEnergy :type "Float (double-precision)")))

(fn `AddEnergy`
  (params (SizeEnergy :type "Float (double-precision)"))
  (returns (EnergyApplied :type "Float (double-precision)"))
  (locals (NextEnergy :type "Float (double-precision)") (PreviouslyEnergy :type "Float (double-precision)"))
  (bind (_current _sizemax) (`self.GetStatsEnergy`))
  (bind ((`EnergySizeCurrent_46_557796174B08A89FF0DB3288A23BCA6E` _energysizecurrent)) (break `/Game/Data/CharacterData1` (`self.CharacterInfo`)))
  (`/Engine/EditorBlueprintResources/ActorMacros.Switch Has Authority`
    (:`Authority`
      (bind _output_get (set `local.NextEnergy` (+ SizeEnergy _current)))
      (if (< _output_get 0.0)
        (set `local.NextEnergy` 0.0)
        (elif (not (<= _output_get _sizemax))
          (set `local.NextEnergy` _sizemax)))
      (bind _output_get_2 (set `local.PreviouslyEnergy` _energysizecurrent))
      (if (== _output_get_2 (`local.NextEnergy`))
        (return 0.0)
        (else
          (`|VariableSetRef` _energysizecurrent (`local.NextEnergy`))
          (`self.UpdateUserInfoWiget`)
          (`self.AddedEnergy` (`local.NextEnergy`) (`local.PreviouslyEnergy`))
          (return (- (`local.NextEnergy`) (`local.PreviouslyEnergy`))))))))

(fn `AddLevelStat`
  (params (StatName :type "/Game/Data/Stats/StatsEnum Enum" :default "NewEnumerator24") (Size :type Integer :default 1))
  (locals (StatData :type "/Game/Data/Stats/StatsItem Structure"))
  (bind (_characterinfo_nickname _characterinfo_level _characterinfo_transform _characterinfo_pointrespawn _characterinfo_charactertype _characterinfo_darkenergy _characterinfo_iapatches _characterinfo_datasize _characterinfo_bagitems _characterinfo_energy _characterinfo_stats) (break `/Game/Data/CharacterData1` (`self.CharacterInfo`)))
  (`/Engine/EditorBlueprintResources/ActorMacros.Switch Has Authority`
    (:`Authority`
      (for (_ _array_index) _characterinfo_stats
        (bind ((`Stats_21_FAA987F240C4D4765694CDA73C34F356` _stats) (`ValueLevelCurrent_9_2356BB8946DB7A675621418CB3ACA55B` _valuelevelcurrent)) (break `/Game/Data/Stats/StatsItem` (`|GetArrayItem` _characterinfo_stats _array_index)))
        (if (`|EnumEquality` _stats (`local.StatName`))
          (`|VariableSetRef` _valuelevelcurrent (+ _valuelevelcurrent (`local.Size`)))
          (return))))))

(fn `AddLevelStatsGroupByIndex`
  (params (Index :type Integer))
  (bind (_characterinfo_nickname _characterinfo_level _characterinfo_transform _characterinfo_pointrespawn _characterinfo_charactertype _characterinfo_darkenergy _characterinfo_iapatches _characterinfo_datasize _characterinfo_bagitems _characterinfo_energy _characterinfo_stats _characterinfo_statsgroups) (break `/Game/Data/CharacterData1` (`self.CharacterInfo`)))
  (bind (_namegroup _statslist _incrementlevel) (break `/Game/Data/Stats/StatsGroups` (`|GetArrayItem` _characterinfo_statsgroups Index)))
  (`/Engine/EditorBlueprintResources/ActorMacros.Switch Has Authority`
    (:`Authority`
      (bind _result (`/Engine/EditorBlueprintResources/StandardMacros.DecrementInt` _characterinfo_darkenergy)
        (:`  `
          (if (< _result 0)
            (`|VariableSetRef` _characterinfo_darkenergy)
            (else
              (for (_array_element _array_index) _statslist
                (`self.AddLevelStat` _array_element (`|GetArrayItem` _incrementlevel _array_index)))
              (`self.UpdateStatsValue`)
              (`|ExecutionSequence`
                (:`then_0`
                  (`self.UpdateStatsWiget`))
                (:`then_1`
                  (`self.UpdateBagWiget`))
                (:`then_2`
                  (`self.UpdateUserInfoWiget`))))))))
    (:`Remote`
      (`self.ServerAddLevelStatsGroupByIndex` Index))))

(fn `AddSkillLevel`
  (params (Skill :type "/Game/Data/Skills/SkillsEnum Enum" :default "NewEnumerator0"))
  (locals (SkillLevel :type Integer))
  (bind _skill (`local.Skill`))
  (bind ((`IAPatches_35_C3979C3E43A2FE95F15DE98B41BFD762` _iapatches)) (break `/Game/Data/CharacterData1` (`self.CharacterInfo`)))
  (bind ((`PointRespawn_82_55D78C5C4C9C365BBAFF1F9AE69BA5F7` _pointrespawn) (`Skills_78_2B1F674E41A77ECED61DFAB1DF2C43E7` _skills)) (break `/Game/Data/CharacterData1` (`self.CharacterInfo`)))
  (`/Engine/EditorBlueprintResources/ActorMacros.Switch Has Authority`
    (:`Authority`
      (if (> _iapatches 0)
        (for (_ _array_index) _skills
          (bind (_skills_2 _level) (break `/Game/Data/Skills/SkillsItem` (`|GetArrayItem` _skills _array_index)))
          (if (`|EnumEquality` _skills_2 _skill)
            (bind _asglobal_game_instance (cast `/Game/Blueprints/GlobalGameInstance` (`GameplayStatics.GetGameInstance`)))
            (bind (_info _good) (`/Game/Blueprints/GlobalGameInstance.GetInfoSkill` _asglobal_game_instance (`local.Skill`)))
            (if _good
              (if (< _level (`KismetMathLibrary.FTrunc` (`.MaxValue_12_D622E5FB4ECD76AD43441C9CEDFA46EC` (break `/Game/Data/ItemInfo` _info))))
                (`/Engine/EditorBlueprintResources/StandardMacros.IncrementInt` _level
                  (:`  `
                    (`/Engine/EditorBlueprintResources/StandardMacros.DecrementInt` _iapatches :!label _label
                      (:`  `
                        _))))))
            (`self.UpdateIAWiget`)
            (`self.UpdateBagWiget`)
            (return)))
        (`KismetArrayLibrary.Array_Add` _skills (make `/Game/Data/Skills/SkillsItem` _skill 1))
        (goto _label)))
    (:`Remote`
      (`self.ServerAddSkillLevel` Skill))))

(fn `GetBagItem`
  (params (Name :type "/Game/Data/Bag/BagItemsEnum Enum" :default "NewEnumerator0"))
  (returns (BagItem :type "/Game/Data/Bag/BagItem Structure") (Good :type Boolean))
  (bind (_characterinfo_nickname _characterinfo_level _characterinfo_transform _characterinfo_pointrespawn _characterinfo_charactertype _characterinfo_darkenergy _characterinfo_iapatches _characterinfo_datasize _characterinfo_bagitems) (break `/Game/Data/CharacterData1` (`self.CharacterInfo`)))
  (for _array_element _characterinfo_bagitems
    (if (`|EnumEquality` (`.Bag_11_B735A13441F558D9CCFDEDAFA4C8AA13` (break `/Game/Data/Bag/BagItem` _array_element)) Name)
      (return _array_element true)))
  (return (struct) false))

(fn `GetSkillLevel`
  (params (Skill :type "/Game/Data/Skills/SkillsEnum Enum" :default "NewEnumerator4"))
  (returns (Level :type Integer))
  (for _array_element (`.Skills_78_2B1F674E41A77ECED61DFAB1DF2C43E7` (break `/Game/Data/CharacterData1` (`self.CharacterInfo`)))
    (bind (_skills _level) (break `/Game/Data/Skills/SkillsItem` _array_element))
    (if (`|EnumEquality` Skill _skills)
      (return _level)))
  (return 0))

(fn `GetStatsCondencator`
  (returns (Current :type "Float (double-precision)") (SizeMax :type "Float (double-precision)") (RecoverySpeed :type "Float (double-precision)"))
  (bind (_characterinfo_nickname _characterinfo_level _characterinfo_transform _characterinfo_pointrespawn _characterinfo_charactertype _characterinfo_darkenergy _characterinfo_iapatches _characterinfo_datasize _characterinfo_bagitems _characterinfo_energy _characterinfo_stats _characterinfo_statsgroups _characterinfo_lasttimerecharge _characterinfo_energysizecurrent _characterinfo_condencatorsizecurrent) (break `/Game/Data/CharacterData1` (`self.CharacterInfo`)))
  (return _characterinfo_condencatorsizecurrent (`.Value_18_A88342054FD7F648EDD54F91339E9EFC` (break `/Game/Data/Stats/StatsItem` (`self.GetStatsData` "NewEnumerator4"))) (`.Value_18_A88342054FD7F648EDD54F91339E9EFC` (break `/Game/Data/Stats/StatsItem` (`self.GetStatsData` "NewEnumerator5")))))

(fn `GetStatsData`
  (params (Stat :type "/Game/Data/Stats/StatsEnum Enum" :default "NewEnumerator24"))
  (returns (StatData :type "/Game/Data/Stats/StatsItem Structure") (Good :type Boolean))
  (bind (_characterinfo_nickname _characterinfo_level _characterinfo_transform _characterinfo_pointrespawn _characterinfo_charactertype _characterinfo_darkenergy _characterinfo_iapatches _characterinfo_datasize _characterinfo_bagitems _characterinfo_energy _characterinfo_stats) (break `/Game/Data/CharacterData1` (`self.CharacterInfo`)))
  (for _array_element _characterinfo_stats
    (if (`|EnumEquality` (`.Stats_21_FAA987F240C4D4765694CDA73C34F356` (break `/Game/Data/Stats/StatsItem` _array_element)) Stat)
      (return _array_element true)))
  (return (struct) false))

(fn `GetStatsDefence`
  (returns (Armor :type "Float (double-precision)") (InBlock :type "Float (double-precision)"))
  (return (`.Value_18_A88342054FD7F648EDD54F91339E9EFC` (break `/Game/Data/Stats/StatsItem` (`self.GetStatsData` "NewEnumerator9"))) (`.Value_18_A88342054FD7F648EDD54F91339E9EFC` (break `/Game/Data/Stats/StatsItem` (`self.GetStatsData` "NewEnumerator10")))))

(fn `GetStatsEnergy`
  (returns (Current :type "Float (double-precision)") (SizeMax :type "Float (double-precision)") (RecoveryProcent :type "Float (double-precision)") (RecoverySpeed :type "Float (double-precision)") (FullRecoveryTimeout :type "Float (double-precision)") (FullRecoveryRestoredTime :type "Float (double-precision)") (FullRecoveryTrueUse :type Boolean))
  (bind (_characterinfo_nickname _characterinfo_level _characterinfo_transform _characterinfo_pointrespawn _characterinfo_charactertype _characterinfo_darkenergy _characterinfo_iapatches _characterinfo_datasize _characterinfo_bagitems _characterinfo_energy _characterinfo_stats _characterinfo_statsgroups _characterinfo_lasttimerecharge _characterinfo_energysizecurrent _characterinfo_condencatorsizecurrent _characterinfo_energyfullrecoverlastuse) (break `/Game/Data/CharacterData1` (`self.CharacterInfo`)))
  (bind ((`Value_18_A88342054FD7F648EDD54F91339E9EFC` _value)) (break `/Game/Data/Stats/StatsItem` (`self.GetStatsData` "NewEnumerator3")))
  (bind _returnvalue (`KismetMathLibrary.GetTotalSeconds` (- (`KismetMathLibrary.Now`) _characterinfo_energyfullrecoverlastuse)))
  (return _characterinfo_energysizecurrent (`.Value_18_A88342054FD7F648EDD54F91339E9EFC` (break `/Game/Data/Stats/StatsItem` (`self.GetStatsData` "NewEnumerator0"))) (`.Value_18_A88342054FD7F648EDD54F91339E9EFC` (break `/Game/Data/Stats/StatsItem` (`self.GetStatsData` "NewEnumerator1"))) (`.Value_18_A88342054FD7F648EDD54F91339E9EFC` (break `/Game/Data/Stats/StatsItem` (`self.GetStatsData` "NewEnumerator2"))) _value _returnvalue (<= _value _returnvalue)))

(fn `GetStatsIA`
  (returns (Level :type "Float (double-precision)") (Energy :type "Float (double-precision)"))
  (return (`.Value_18_A88342054FD7F648EDD54F91339E9EFC` (break `/Game/Data/Stats/StatsItem` (`self.GetStatsData` "NewEnumerator19"))) (`.Value_18_A88342054FD7F648EDD54F91339E9EFC` (break `/Game/Data/Stats/StatsItem` (`self.GetStatsData` "NewEnumerator20")))))

(fn `GetStatsKick`
  (returns (Size :type "Float (double-precision)") (TimeoutMultiply :type "Float (double-precision)"))
  (return (`.Value_18_A88342054FD7F648EDD54F91339E9EFC` (break `/Game/Data/Stats/StatsItem` (`self.GetStatsData` "NewEnumerator11"))) (`.Value_18_A88342054FD7F648EDD54F91339E9EFC` (break `/Game/Data/Stats/StatsItem` (`self.GetStatsData` "NewEnumerator12")))))

(fn `GetStatsRocket`
  (returns (Power :type "Float (double-precision)") (Speed :type "Float (double-precision)") (MaxDistanceFly :type "Float (double-precision)") (ExplosionDistance :type "Float (double-precision)") (RechargeTimeout :type "Float (double-precision)") (TimeAiming :type "Float (double-precision)") (GradusCorrection :type "Float (double-precision)"))
  (return (`.Value_18_A88342054FD7F648EDD54F91339E9EFC` (break `/Game/Data/Stats/StatsItem` (`self.GetStatsData` "NewEnumerator13"))) (`.Value_18_A88342054FD7F648EDD54F91339E9EFC` (break `/Game/Data/Stats/StatsItem` (`self.GetStatsData` "NewEnumerator14"))) (`.Value_18_A88342054FD7F648EDD54F91339E9EFC` (break `/Game/Data/Stats/StatsItem` (`self.GetStatsData` "NewEnumerator15"))) (`.Value_18_A88342054FD7F648EDD54F91339E9EFC` (break `/Game/Data/Stats/StatsItem` (`self.GetStatsData` "NewEnumerator16"))) (`.Value_18_A88342054FD7F648EDD54F91339E9EFC` (break `/Game/Data/Stats/StatsItem` (`self.GetStatsData` "NewEnumerator17"))) (`.Value_18_A88342054FD7F648EDD54F91339E9EFC` (break `/Game/Data/Stats/StatsItem` (`self.GetStatsData` "NewEnumerator23"))) (`.Value_18_A88342054FD7F648EDD54F91339E9EFC` (break `/Game/Data/Stats/StatsItem` (`self.GetStatsData` "NewEnumerator18")))))

(fn `GetStatsSpeed`
  (returns (Walk :type "Float (double-precision)") (Run :type "Float (double-precision)") (SuperRun :type "Float (double-precision)"))
  (return (`.Value_18_A88342054FD7F648EDD54F91339E9EFC` (break `/Game/Data/Stats/StatsItem` (`self.GetStatsData` "NewEnumerator6"))) (`.Value_18_A88342054FD7F648EDD54F91339E9EFC` (break `/Game/Data/Stats/StatsItem` (`self.GetStatsData` "NewEnumerator7"))) (`.Value_18_A88342054FD7F648EDD54F91339E9EFC` (break `/Game/Data/Stats/StatsItem` (`self.GetStatsData` "NewEnumerator8")))))

(fn `Process`
  (locals (CallInterval :type "Float (double-precision)"))
  (bind (_current _sizemax _recoveryprocent _recoveryspeed) (`self.GetStatsEnergy`))
  (bind (_current_2 _sizemax_2 _recoveryspeed_2) (`self.GetStatsCondencator`))
  (bind (_characterinfo_nickname _characterinfo_level _characterinfo_transform _characterinfo_pointrespawn _characterinfo_charactertype _characterinfo_darkenergy _characterinfo_iapatches _characterinfo_datasize _characterinfo_bagitems _characterinfo_energy _characterinfo_stats _characterinfo_statsgroups _characterinfo_lasttimerecharge) (break `/Game/Data/CharacterData1` (`self.CharacterInfo`)))
  (bind ((`CondencatorSizeCurrent_48_2F4CFB71414F704B55373295F615E1B8` _condencatorsizecurrent)) (break `/Game/Data/CharacterData1` (`self.CharacterInfo`)))
  (bind _returnvalue (+ _current_2 (* (`local.CallInterval`) _recoveryspeed_2)))
  ;[1 0.9696 0.5955] Calculate and update time
  (`/Engine/EditorBlueprintResources/ActorMacros.Switch Has Authority`
    (:`Authority`
      (set `local.CallInterval` (`KismetMathLibrary.GetTotalSeconds` (- (`KismetMathLibrary.Now`) _characterinfo_lasttimerecharge)))
      (`|VariableSetRef` _characterinfo_lasttimerecharge (`KismetMathLibrary.Now`))
      (`|ExecutionSequence`
        (:`then_0`
          ;[1 0.3851 0.405] Increment energy current value
          (if (< _current (* _sizemax _recoveryprocent))
            (`self.AddEnergy` (* (`local.CallInterval`) _recoveryspeed))))
        (:`then_1`
          ;[0.3915 0.4731 1] Increment condencator current value
          (if (> _returnvalue _sizemax_2)
            (`|VariableSetRef` _condencatorsizecurrent _sizemax_2)
            (else
              (`|VariableSetRef` _condencatorsizecurrent _returnvalue))))
        (:`then_2`
          (`self.UpdateUserInfoWiget` :!label _label))))
    (:`Remote`
      (goto _label))))

(fn `RespawnCharacter`
  (params (RegenerateEnergy :type Boolean))
  (`parent.RespawnCharacter` RegenerateEnergy)
  (if RegenerateEnergy
    (`GameplayStatics.ApplyDamage` self -100000.0)))

(fn `TakeInBag`
  (params (Name :type "/Game/Data/Bag/BagItemsEnum Enum" :default "NewEnumerator0") (Size :type Integer))
  (locals (BagItem :type "/Game/Data/Bag/BagItem Structure"))
  (bind (_characterinfo_nickname _characterinfo_level _characterinfo_transform _characterinfo_pointrespawn _characterinfo_charactertype _characterinfo_darkenergy _characterinfo_iapatches _characterinfo_datasize _characterinfo_bagitems) (break `/Game/Data/CharacterData1` (`self.CharacterInfo`)))
  (`/Engine/EditorBlueprintResources/ActorMacros.Switch Has Authority`
    (:`Authority`
      (if (> Size 0)
        (for (_ _array_index) _characterinfo_bagitems
          (bind (_bag _size) (break `/Game/Data/Bag/BagItem` (`|GetArrayItem` _characterinfo_bagitems _array_index)))
          (if (`|EnumEquality` _bag (`local.Name`))
            (`|VariableSetRef` _size (+ _size (`local.Size`)))
            (`self.UpdateBagWiget`)
            (return)))
        (`KismetArrayLibrary.Array_Add` _characterinfo_bagitems (make `/Game/Data/Bag/BagItem` (`local.Name`) (`local.Size`)))
        (return)))))

(fn `TakeOutBag`
  (params (Name :type "/Game/Data/Bag/BagItemsEnum Enum" :default "NewEnumerator0") (Size :type Integer))
  (returns (Have :type Boolean) (ResultSize :type Integer))
  (bind (_characterinfo_nickname _characterinfo_level _characterinfo_transform _characterinfo_pointrespawn _characterinfo_charactertype _characterinfo_darkenergy _characterinfo_iapatches _characterinfo_datasize _characterinfo_bagitems) (break `/Game/Data/CharacterData1` (`self.CharacterInfo`)))
  (bind (_characterinfo_nickname_2 _characterinfo_level_2 _characterinfo_transform_2 _characterinfo_pointrespawn_2 _characterinfo_charactertype_2 _characterinfo_darkenergy_2 _characterinfo_iapatches_2 _characterinfo_datasize_2 _characterinfo_bagitems_2) (break `/Game/Data/CharacterData1` (`self.CharacterInfo`)))
  (`/Engine/EditorBlueprintResources/ActorMacros.Switch Has Authority`
    (:`Authority`
      (if (> Size 0)
        (for (_ _array_index) _characterinfo_bagitems
          (bind _output (`|GetArrayItem` _characterinfo_bagitems _array_index))
          (bind (_bag _size) (break `/Game/Data/Bag/BagItem` _output))
          (if (`|EnumEquality` _bag (`local.Name`))
            (bind _returnvalue (- _size (`local.Size`)))
            (if (>= _returnvalue 0)
              (`|VariableSetRef` _size _returnvalue)
              (if (== _size 0)
                (`KismetArrayLibrary.Array_RemoveItem` _characterinfo_bagitems_2 _output))
              (return true 0)
              (else
                (return false (* _returnvalue -1))))))
        (return false (`local.Size`))))))

(fn `UpdateBagWiget`
  (bind _wbbag (`self.WBBag`))
  (set `self.NeedUpdateUI` true)
  (`/Engine/EditorBlueprintResources/StandardMacros.IsValid` _wbbag
    (:`Is Valid`
      (`/Game/UI/WidgetBlueprint/GameLevel/WBUpdate.Update` _wbbag))))

(fn `UpdateIAWiget`
  (bind _wbia (`self.WBIA`))
  (set `self.NeedUpdateUI` true)
  (`/Engine/EditorBlueprintResources/StandardMacros.IsValid` _wbia
    (:`Is Valid`
      (`/Game/UI/WidgetBlueprint/GameLevel/WBUpdate.Update` _wbia))))

(fn `UpdateStatsValue`
  (locals (StatData :type "/Game/Data/Stats/StatsItem Structure"))
  (bind (_characterinfo_nickname _characterinfo_level _characterinfo_transform _characterinfo_pointrespawn _characterinfo_charactertype _characterinfo_darkenergy _characterinfo_iapatches _characterinfo_datasize _characterinfo_bagitems _characterinfo_energy _characterinfo_stats) (break `/Game/Data/CharacterData1` (`self.CharacterInfo`)))
  (`/Engine/EditorBlueprintResources/ActorMacros.Switch Has Authority`
    (:`Authority`
      (for (_ _array_index) _characterinfo_stats
        (`self.UpdateValue` (`|GetArrayItem` _characterinfo_stats _array_index))))))

(fn `UpdateStatsWiget`
  (bind _wbstats (`self.WBStats`))
  (set `self.NeedUpdateUI` true)
  (`/Engine/EditorBlueprintResources/StandardMacros.IsValid` _wbstats
    (:`Is Valid`
      (`/Game/UI/WidgetBlueprint/GameLevel/WBUpdate.Update` _wbstats))))

(fn `UpdateUserInfoWiget`
  (bind _wbuserinfo (`self.WBUserInfo`))
  (set `self.NeedUpdateUI` true)
  (`/Engine/EditorBlueprintResources/StandardMacros.IsValid` _wbuserinfo
    (:`Is Valid`
      (`/Game/UI/WidgetBlueprint/GameLevel/WBUpdate.Update` _wbuserinfo))))

(fn `UpdateValue`
  (params (Info :type "/Game/Data/Stats/StatsItem Structure (by ref)"))
  (bind (_stats _valuebase _valuelevelcurrent _valuestepforitemlevel _valuestepforcharacterlevel _value) (break `/Game/Data/Stats/StatsItem` Info))
  (bind (_characterinfo_nickname _characterinfo_level) (break `/Game/Data/CharacterData1` (`self.CharacterInfo`)))
  (`|VariableSetRef` _value (+ _valuebase (* _valuelevelcurrent _valuestepforitemlevel) (* (`KismetMathLibrary.FTrunc` _characterinfo_level) _valuestepforcharacterlevel)))
  (return))

(fn `UseBagItem`
  (params (Name :type "/Game/Data/Bag/BagItemsEnum Enum" :default "NewEnumerator0"))
  (locals (BagItem :type "/Game/Data/Bag/BagItem Structure"))
  (`/Engine/EditorBlueprintResources/ActorMacros.Switch Has Authority`
    (:`Authority`
      (bind (_bagitem _good) (`self.GetBagItem` Name))
      (if (`.MinusOnUse_8_B68ABCD04B6F55309B59F2B534148BA0` (break `/Game/Data/Bag/BagItem` _bagitem))
        (if _good
          (`self.TakeOutBag` (`local.Name`) 1)
          ;[1 1 1] Do somthing item (use)
          (`self.UpdateBagWiget`))))
    (:`Remote`
      (`self.ServerUseBagItem` Name))))

(fn `UseCondencator`
  (params (UsedSize :type "Float (double-precision)"))
  (returns (Successful :type Boolean))
  (bind (_characterinfo_nickname _characterinfo_level _characterinfo_transform _characterinfo_pointrespawn _characterinfo_charactertype _characterinfo_darkenergy _characterinfo_iapatches _characterinfo_datasize _characterinfo_bagitems _characterinfo_energy _characterinfo_stats _characterinfo_statsgroups _characterinfo_lasttimerecharge _characterinfo_energysizecurrent _characterinfo_condencatorsizecurrent) (break `/Game/Data/CharacterData1` (`self.CharacterInfo`)))
  (`/Engine/EditorBlueprintResources/ActorMacros.Switch Has Authority`
    (:`Authority`
      (if (and (>= UsedSize 0.0) (<= UsedSize _characterinfo_condencatorsizecurrent))
        (`|VariableSetRef` _characterinfo_condencatorsizecurrent (- _characterinfo_condencatorsizecurrent UsedSize))
        (`self.UpdateUserInfoWiget`)
        (return true)
        (else
          (return false))))))

(fn `UserConstructionScript`
  (`parent.UserConstructionScript`))